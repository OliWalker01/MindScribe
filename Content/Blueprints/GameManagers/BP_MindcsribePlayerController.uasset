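; Player controller that records Maths Blitz results (player name, score, difficulty) through its SetMathsBlitzScore event.
; It creates a new BP_GameSave, writing it to the MathsBlitzScore slot only if loading that slot fails; a loaded save is never used.
; The result is inserted before the first entry it ties or beats, then all entries are printed.
; The updated list is not saved afterwards.
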(event Custom|Set%20Maths%20Blitz%20Score
  (params (PlayerString :type String) (Last%20Score :type Integer) (Difficulty :type String))
  (Variables|Default|SetLastScore Last%20Score)
  (Variables|Default|SetDifficulty Difficulty)
  (Utilities|FlowControl|Sequence
    (:then_0
      (Variables|Default|SetNewMathsBlitzStruct (Utilities|Struct|MakeStruct_MathsBlitz (Variables|Default|GetPlayerName) (Variables|Default|GetLastScore) (Variables|Default|GetDifficulty)))
      (bind _returnvalue (SaveGame|CreateSaveGameObject "/Game/Blueprints/GameManagers/BP_GameSave.BP_GameSave_C"))
      (Variables|Default|SetGameSaveRef _returnvalue)
      (bind _returnvalue_2 (SaveGame|LoadGamefromSlot "MathsBlitzScore"))
      (Utilities|IsValid _returnvalue_2
        (:Is%20Not%20Valid
          (SaveGame|SaveGametoSlot (Variables|Default|GetGameSaveRef) "MathsBlitzScore"))))
    (:then_1
      (bind (_array_element _array_index) (Utilities|Array|ForEachLoopwithBreak (Variables|/Game/Blueprints/GameManagers/BP_GameSave.BP_GameSave_C|GetMaths%20Blitz%20Struct (Variables|Default|GetGameSaveRef)) :!label _label)
        (:LoopBody
          (if (not (> (.score _array_element) (Variables|Default|GetLastScore)))
            (Utilities|Array|Insert (Variables|/Game/Blueprints/GameManagers/BP_GameSave.BP_GameSave_C|GetMaths%20Blitz%20Struct (Variables|Default|GetGameSaveRef)) (Variables|Default|GetNewMathsBlitzStruct) _array_index)
            (goto _label Break)))
        (:Completed
          (for _array_element_2 (Variables|/Game/Blueprints/GameManagers/BP_GameSave.BP_GameSave_C|GetMaths%20Blitz%20Struct (Variables|Default|GetGameSaveRef))
            (Development|PrintString (Utilities|String|Append "PlayerName: " (.playername _array_element_2)))
            (Development|PrintString (Utilities|String|Append "Score: " (Utilities|String|ToString(Integer) (.score _array_element_2))))
            (Development|PrintString (Utilities|String|Append "Difficulty: " (.difficulty _array_element_2)))))))))

(fn ConstructionScript)