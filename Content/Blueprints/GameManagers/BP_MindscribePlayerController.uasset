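; BP_MindscribePlayerController is a player controller that persists Maths Blitz scores through a BP_GameSave object in the "Scores" slot.
; On BeginPlay it loads the existing save and copies the Easy, Medium and Hard score arrays into its own variables, or creates and saves a new one.
; SaveMathsBlitzScores writes those arrays back to the slot.
; Debug prints show loaded Easy scores and whether saving succeeded.
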(event Custom|Set%20Maths%20Blitz%20Scores
  (bind _gamesaveref (Variables|Default|GetGameSaveRef))
  ;[1 1 1] Sets the Scores for Maths Blitz
  (Variables|MathsBlitz|SetMathsBlitzScoresEasy (Variables|/Game/Blueprints/GameManagers/BP_GameSave.BP_GameSave_C|GetMathsBlitzEasyScores _gamesaveref))
  (Variables|MathsBlitz|SetMathsBlitzScoresMedium (Variables|/Game/Blueprints/GameManagers/BP_GameSave.BP_GameSave_C|GetMathsBlitzMediumScores _gamesaveref))
  (Variables|MathsBlitz|SetMathsBlitzScoresHard (Variables|/Game/Blueprints/GameManagers/BP_GameSave.BP_GameSave_C|GetMathsBlitzHardScores _gamesaveref)))

(event Custom|Save%20Maths%20Blitz%20Scores
  (bind _gamesaveref (Variables|Default|GetGameSaveRef))
  ;[1 1 1] Saves Maths Blitz Scores
  (Variables|/Game/Blueprints/GameManagers/BP_GameSave.BP_GameSave_C|SetMathsBlitzEasyScores _gamesaveref (Variables|MathsBlitz|GetMathsBlitzScoresEasy))
  (Variables|/Game/Blueprints/GameManagers/BP_GameSave.BP_GameSave_C|SetMathsBlitzMediumScores _gamesaveref (Variables|MathsBlitz|GetMathsBlitzScoresMedium))
  (Variables|/Game/Blueprints/GameManagers/BP_GameSave.BP_GameSave_C|SetMathsBlitzHardScores _gamesaveref (Variables|MathsBlitz|GetMathsBlitzScoresHard))
  (bind _returnvalue (SaveGame|SaveGametoSlot (Variables|Default|GetGameSaveRef) "Scores"))
  (if _returnvalue
    (Development|PrintString "Game Saved")
    (else
      (Development|PrintString "Game Not Saved"))))

(event EventBeginPlay
  (bind _returnvalue (SaveGame|DoesSaveGameExist "Scores"))
  (if _returnvalue
    (bind _returnvalue_2 (SaveGame|LoadGamefromSlot "Scores"))
    (bind _asbp_game_save (Utilities|Casting|CastToBP_GameSave _returnvalue_2))
    (Variables|Default|SetGameSaveRef _asbp_game_save)
    (CallFunction|SetMathsBlitzScores)
    (for _array_element (Variables|MathsBlitz|GetMathsBlitzScoresEasy)
      (Development|PrintString (Utilities|String|Append "Player Score: " (Utilities|String|ToString(Integer) _array_element))))
    (else
      (bind _returnvalue_3 (SaveGame|CreateSaveGameObject "/Game/Blueprints/GameManagers/BP_GameSave.BP_GameSave_C"))
      (bind _output_get (Variables|Default|SetGameSaveRef _returnvalue_3))
      (SaveGame|SaveGametoSlot _output_get "Scores"))))

(fn ConstructionScript)