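; BP_Screen is a screen actor in a VR maths game that generates random arithmetic questions and builds the player's typed answer.
; MathsQuestion reads the VR_Player's difficulty and routes Easy to an addition generator that splits a random target into two operands.
; MediumQuestion picks addition or non-negative subtraction, but this switch does not call it.
; UpdatePlayerInput appends selected digits, and GetScreen loads a widget onto the screen.
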(event Custom|Easy%20Question
  ;[1 1 1] Calculates a Random Sum - Easy
  (Utilities|FlowControl|Delay 0.2)
  (Variables|Default|SetPlayer%20Inputted? false)
  (Variables|MathsGame|SetMaths%20Symbol "+")
  (bind _output_get (Variables|MathsGame|SetTarget%20Number (Math|Random|RandomIntegerinRange 0 25)))
  (Variables|MathsGame|SetNumber%20One (- _output_get (Math|Random|RandomIntegerinRange 0 (Variables|MathsGame|GetTarget%20Number))))
  (Variables|MathsGame|SetNumber%20Two (- (Variables|MathsGame|GetTarget%20Number) (Variables|MathsGame|GetNumber%20One))))

(event Custom|Get%20Screen
  (bind _returnvalue (UserInterface|CreateWidget "/Game/Assets/Widgets/Widget_Menu.Widget_Menu_C"))
  (UserInterface|SetWidget (Variables|Default|GetWidget) _returnvalue))

(event Custom|Maths%20Question
  (switch string (Variables|/Game/Blueprints/VR_Player.VR_Player_C|GetDifficulty (Variables|Default|GetPlayer%20Ref))
    (:Easy
      (CallFunction|EasyQuestion))))

(event Custom|Medium%20Question
  ;[1 1 1] Calculates A Random Sum - Medium
  (Utilities|FlowControl|Delay 0.2)
  (Variables|Default|SetPlayer%20Inputted? false)
  (switch int (Math|Random|RandomIntegerinRange 0 1)
    (:0
      (Variables|MathsGame|SetMaths%20Symbol "+")
      (Variables|MathsGame|SetNumber%20One (Math|Random|RandomIntegerinRange 0 25))
      (Variables|MathsGame|SetNumber%20Two (Math|Random|RandomIntegerinRange 0 25))
      (Variables|MathsGame|SetTarget%20Number (+ (Variables|MathsGame|GetNumber%20One) (Variables|MathsGame|GetNumber%20Two))))
    (:1
      (Variables|MathsGame|SetMaths%20Symbol "-")
      (bind _output_get (Variables|MathsGame|SetNumber%20One (Math|Random|RandomIntegerinRange 0 25)))
      (Variables|MathsGame|SetNumber%20Two (Math|Random|RandomIntegerinRange 0 _output_get))
      (Variables|MathsGame|SetTarget%20Number (- (Variables|MathsGame|GetNumber%20One) (Variables|MathsGame|GetNumber%20Two))))))

(event EventBeginPlay
  ;[1 1 1] Sets Object References
  (bind _returnvalue (Actor|GetActorOfClass "/Game/Blueprints/VR_Player.VR_Player_C"))
  (Variables|Default|SetPlayer%20Ref _returnvalue))

(event EventUpdatePlayerInput
  (params (Number%20Selected :type Integer))
  ;[1 1 1] Updates Player Input Number Depending On What Number Is Selected
  (Variables|Default|SetPlayer%20Inputted? true)
  (if (!= (Variables|MathsGame|GetPlayer%20Inputted%20Number) 0)
    (Variables|MathsGame|SetPlayer%20Inputted%20Number (+ (* (Variables|MathsGame|GetPlayer%20Inputted%20Number) 10) Number%20Selected))
    (else
      (Variables|MathsGame|SetPlayer%20Inputted%20Number Number%20Selected))))

(fn ConstructionScript)