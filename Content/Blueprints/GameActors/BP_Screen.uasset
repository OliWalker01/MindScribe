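; BP_Screen is a screen actor that hosts a player ID widget and records numeric input from the player.
; GetScreen creates the Widget_PlayerID widget and assigns it to the actor's widget component.
; UpdatePlayerInput flags that input occurred and appends each selected digit by multiplying the stored number by ten and adding it.
; BeginPlay caches a reference to the BP_VR_Player actor.
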(event Custom|Get%20Screen
  ;[1 1 1] Screen Reference
  (bind _returnvalue (UserInterface|CreateWidget "/Game/Widgets/Widget_PlayerID.Widget_PlayerID_C"))
  (UserInterface|SetWidget (Variables|Default|GetWidget) _returnvalue))

(event EventBeginPlay
  ;[1 1 1] Sets Object References
  (bind _returnvalue (Actor|GetActorOfClass "/Game/Blueprints/GameActors/BP_VR_Player.BP_VR_Player_C"))
  (Variables|Default|SetPlayer%20Ref _returnvalue))

(event EventUpdatePlayerInput
  (params (Number%20Selected :type Integer))
  ;[1 1 1] Updates Player Input Number Depending On What Number Is Selected
  (Variables|Default|SetPlayer%20Inputted? true)
  (if (!= (Variables|MathsGame|GetPlayer%20Inputted%20Number) 0)
    (Variables|MathsGame|SetPlayer%20Inputted%20Number (+ (* (Variables|MathsGame|GetPlayer%20Inputted%20Number) 10) Number%20Selected))
    (else
      (Variables|MathsGame|SetPlayer%20Inputted%20Number Number%20Selected))))

(fn ConstructionScript)