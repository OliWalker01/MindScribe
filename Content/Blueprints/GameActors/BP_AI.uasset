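; BP_AI is an actor for the AI opponent in the SnapIt game, holding its score and difficulty and deciding when the game ends.
; On BeginPlay it caches the BP_Screen actor to read the player's score.
; CheckSnapItScore quits the application when either score reaches a fixed target on Easy, or when the player reaches a set lead over the AI on Medium and Hard.
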(event Custom|Check%20Snap%20It%20Score
  (switch string (Variables|Default|GetDifficulty)
    (:Easy
      (if (or (>= (Variables|/Game/Blueprints/GameActors/BP_Screen.BP_Screen_C|GetSnapItPlayerScore (Variables|Default|GetScreen%20Ref)) 5) (>= (Variables|Default|GetaiScore) 5))
        (Game|QuitGame 0 "Quit" false :!label _label)))
    (:Medium
      (if (>= (Variables|/Game/Blueprints/GameActors/BP_Screen.BP_Screen_C|GetSnapItPlayerScore (Variables|Default|GetScreen%20Ref)) (+ (Variables|Default|GetaiScore) 3))
        (goto _label)))
    (:Hard
      (if (>= (Variables|/Game/Blueprints/GameActors/BP_Screen.BP_Screen_C|GetSnapItPlayerScore (Variables|Default|GetScreen%20Ref)) (+ (Variables|Default|GetaiScore) 5))
        (goto _label)))))

(event EventBeginPlay
  (bind _returnvalue (Actor|GetActorOfClass "/Game/Blueprints/GameActors/BP_Screen.BP_Screen_C"))
  (Variables|Default|SetScreen%20Ref _returnvalue))

(fn ConstructionScript)