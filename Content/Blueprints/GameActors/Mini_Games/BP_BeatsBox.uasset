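; BP_BeatsBox is a VR piano memory mini-game where the player repeats a sequence of four lit, sounding keys.
; Each round PickPianoSequence builds and plays a fresh sequence, then opens the player's turn.
; Motion controller overlaps record notes through per-key DoOnce gates, and end overlaps check the answer once it is long enough.
; Success lengthens the next sequence; failure saves the sorted score on the player controller and shows the scoreboard on BP_Screen.
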(event OnComponentBeginOverlap(B_Note_Box_Collison)
  (params (OverlappedComponent :type Primitive%20Component%20Object%20Reference) (OtherActor :type Actor%20Object%20Reference) (OtherComp :type Primitive%20Component%20Object%20Reference) (OtherBodyIndex :type Integer) (bFromSweep :type Boolean) (SweepResult :type Hit%20Result%20Structure%20%28by%20ref%29))
  (bind _player_ref (Variables|Default|GetPlayer%20Ref))
  (if (or (== OtherComp (Variables|/Game/Blueprints/GameActors/BP_VR_Player.BP_VR_Player_C|GetMotion%20Controller%20Left%20Collision _player_ref)) (== OtherComp (Variables|/Game/Blueprints/GameActors/BP_VR_Player.BP_VR_Player_C|GetMotion%20Controller%20Right%20Collision _player_ref)))
    (if (Variables|Default|GetPlayerTurn?)
      (Utilities|FlowControl|DoOnce false
        (:Completed
          (Audio|SpawnSound2D "/Game/Assets/Audio/PianNotes/SoundCues/SQ_Piano_B_Note.SQ_Piano_B_Note" 1.0 1.0 0.0 0)
          (Rendering|Material|SetMaterial (Variables|Default|GetB_Note) 0 "/Game/Assets/Textures/M_PianoSelectedKey.M_PianoSelectedKey")
          (Utilities|Array|Add (Variables|Default|GetPlayerAnswer) "B"))))))

(event OnComponentBeginOverlap(A_Note_Box_Collison)
  (params (OverlappedComponent :type Primitive%20Component%20Object%20Reference) (OtherActor :type Actor%20Object%20Reference) (OtherComp :type Primitive%20Component%20Object%20Reference) (OtherBodyIndex :type Integer) (bFromSweep :type Boolean) (SweepResult :type Hit%20Result%20Structure%20%28by%20ref%29))
  (bind _player_ref (Variables|Default|GetPlayer%20Ref))
  (if (or (== OtherComp (Variables|/Game/Blueprints/GameActors/BP_VR_Player.BP_VR_Player_C|GetMotion%20Controller%20Left%20Collision _player_ref)) (== OtherComp (Variables|/Game/Blueprints/GameActors/BP_VR_Player.BP_VR_Player_C|GetMotion%20Controller%20Right%20Collision _player_ref)))
    (if (Variables|Default|GetPlayerTurn?)
      (Utilities|FlowControl|DoOnce false
        (:Completed
          (Audio|SpawnSound2D "/Game/Assets/Audio/PianNotes/SoundCues/SQ_Piano_A_Note.SQ_Piano_A_Note" 1.0 1.0 0.0 0)
          (Rendering|Material|SetMaterial (Variables|Default|GetA_Note) 0 "/Game/Assets/Textures/M_PianoSelectedKey.M_PianoSelectedKey")
          (Utilities|Array|Add (Variables|Default|GetPlayerAnswer) "A"))))))

(event OnComponentEndOverlap(D_Note_Box_Collison)
  (params (OverlappedComponent :type Primitive%20Component%20Object%20Reference) (OtherActor :type Actor%20Object%20Reference) (OtherComp :type Primitive%20Component%20Object%20Reference) (OtherBodyIndex :type Integer))
  (bind _player_ref (Variables|Default|GetPlayer%20Ref))
  (if (or (== OtherComp (Variables|/Game/Blueprints/GameActors/BP_VR_Player.BP_VR_Player_C|GetMotion%20Controller%20Left%20Collision _player_ref)) (== OtherComp (Variables|/Game/Blueprints/GameActors/BP_VR_Player.BP_VR_Player_C|GetMotion%20Controller%20Right%20Collision _player_ref)))
    (if (Variables|Default|GetPlayerTurn?)
      (Utilities|FlowControl|Sequence
        (:then_0
          (Utilities|FlowControl|DoOnce false) ; enters at Reset
        )
        (:then_1
          (Rendering|Material|SetMaterial (Variables|Default|GetD_Note) 0 "/Game/Assets/Textures/M_White.M_White")
          (if (>= (Utilities|Array|Length (Variables|Default|GetPlayerAnswer)) (Utilities|Array|Length (Variables|Default|GetPianoSequence)))
            (bind _correct_ (CallFunction|CheckAnswer))
            (if _correct_
              (Variables|Default|SetPlayerTurn? false)
              (Variables|Default|SetPlayerScore (+ (Variables|Default|GetPlayerScore) 1))
              (Variables|Default|SetSequenceLength (+ (Variables|Default|GetSequenceLength) 1))
              (Utilities|Array|Clear (Variables|Default|GetPlayerAnswer))
              (Utilities|FlowControl|Delay 2.0)
              (CallFunction|PickPianoSequence)
              (else
                (Utilities|Array|Add (Variables|/Game/Blueprints/GameManagers/BP_MindscribePlayerController.BP_MindscribePlayerController_C|GetBeats_Box_Scores (Variables|Default|GetPlayer%20Controller%20Ref)) (Variables|Default|GetPlayerScore))
                (Class|LowEntryExtendedStandardLibrary|SortIntegerArrayDirectly (Variables|/Game/Blueprints/GameManagers/BP_MindscribePlayerController.BP_MindscribePlayerController_C|GetBeats_Box_Scores (Variables|Default|GetPlayer%20Controller%20Ref)) true)
                (Default|SaveBeatsBoxScore (Variables|Default|GetPlayer%20Controller%20Ref))
                (Utilities|FlowControl|Delay 3.0)
                (bind _returnvalue (UserInterface|CreateWidget "/Game/Widgets/BeatsBox/Widget_BeatsBoxScoreboard.Widget_BeatsBoxScoreboard_C"))
                (UserInterface|SetWidget (Variables|/Game/Blueprints/GameActors/BP_Screen.BP_Screen_C|GetWidget (Variables|Default|GetScreen%20Ref)) _returnvalue)))))))))

(event OnComponentBeginOverlap(C_Note_Box_Collison)
  (params (OverlappedComponent :type Primitive%20Component%20Object%20Reference) (OtherActor :type Actor%20Object%20Reference) (OtherComp :type Primitive%20Component%20Object%20Reference) (OtherBodyIndex :type Integer) (bFromSweep :type Boolean) (SweepResult :type Hit%20Result%20Structure%20%28by%20ref%29))
  (bind _player_ref (Variables|Default|GetPlayer%20Ref))
  (if (or (== OtherComp (Variables|/Game/Blueprints/GameActors/BP_VR_Player.BP_VR_Player_C|GetMotion%20Controller%20Left%20Collision _player_ref)) (== OtherComp (Variables|/Game/Blueprints/GameActors/BP_VR_Player.BP_VR_Player_C|GetMotion%20Controller%20Right%20Collision _player_ref)))
    (if (Variables|Default|GetPlayerTurn?)
      (Utilities|FlowControl|DoOnce false
        (:Completed
          (Audio|SpawnSound2D "/Game/Assets/Audio/PianNotes/SoundCues/SQ_Piano_C_Note.SQ_Piano_C_Note" 1.0 1.0 0.0 0)
          (Rendering|Material|SetMaterial (Variables|Default|GetC_Note) 0 "/Game/Assets/Textures/M_PianoSelectedKey.M_PianoSelectedKey")
          (Utilities|Array|Add (Variables|Default|GetPlayerAnswer) "C"))))))

(event OnComponentBeginOverlap(D_Note_Box_Collison)
  (params (OverlappedComponent :type Primitive%20Component%20Object%20Reference) (OtherActor :type Actor%20Object%20Reference) (OtherComp :type Primitive%20Component%20Object%20Reference) (OtherBodyIndex :type Integer) (bFromSweep :type Boolean) (SweepResult :type Hit%20Result%20Structure%20%28by%20ref%29))
  (bind _player_ref (Variables|Default|GetPlayer%20Ref))
  (if (or (== OtherComp (Variables|/Game/Blueprints/GameActors/BP_VR_Player.BP_VR_Player_C|GetMotion%20Controller%20Left%20Collision _player_ref)) (== OtherComp (Variables|/Game/Blueprints/GameActors/BP_VR_Player.BP_VR_Player_C|GetMotion%20Controller%20Right%20Collision _player_ref)))
    (if (Variables|Default|GetPlayerTurn?)
      (Utilities|FlowControl|DoOnce false
        (:Completed
          (Audio|SpawnSound2D "/Game/Assets/Audio/PianNotes/SoundCues/SQ_Piano_D_Note.SQ_Piano_D_Note" 1.0 1.0 0.0 0)
          (Rendering|Material|SetMaterial (Variables|Default|GetD_Note) 0 "/Game/Assets/Textures/M_PianoSelectedKey.M_PianoSelectedKey")
          (Utilities|Array|Add (Variables|Default|GetPlayerAnswer) "D"))))))

(event OnComponentEndOverlap(A_Note_Box_Collison)
  (params (OverlappedComponent :type Primitive%20Component%20Object%20Reference) (OtherActor :type Actor%20Object%20Reference) (OtherComp :type Primitive%20Component%20Object%20Reference) (OtherBodyIndex :type Integer))
  (bind _player_ref (Variables|Default|GetPlayer%20Ref))
  (if (or (== OtherComp (Variables|/Game/Blueprints/GameActors/BP_VR_Player.BP_VR_Player_C|GetMotion%20Controller%20Left%20Collision _player_ref)) (== OtherComp (Variables|/Game/Blueprints/GameActors/BP_VR_Player.BP_VR_Player_C|GetMotion%20Controller%20Right%20Collision _player_ref)))
    (if (Variables|Default|GetPlayerTurn?)
      (Utilities|FlowControl|Sequence
        (:then_0
          (Utilities|FlowControl|DoOnce false) ; enters at Reset
        )
        (:then_1
          (Rendering|Material|SetMaterial (Variables|Default|GetA_Note) 0 "/Game/Assets/Textures/M_White.M_White")
          (if (>= (Utilities|Array|Length (Variables|Default|GetPlayerAnswer)) (Utilities|Array|Length (Variables|Default|GetPianoSequence)))
            (bind _correct_ (CallFunction|CheckAnswer))
            (if _correct_
              (Variables|Default|SetPlayerTurn? false)
              (Variables|Default|SetPlayerScore (+ (Variables|Default|GetPlayerScore) 1))
              (Variables|Default|SetSequenceLength (+ (Variables|Default|GetSequenceLength) 1))
              (Utilities|Array|Clear (Variables|Default|GetPlayerAnswer))
              (Utilities|FlowControl|Delay 2.0)
              (CallFunction|PickPianoSequence)
              (else
                (Utilities|Array|Add (Variables|/Game/Blueprints/GameManagers/BP_MindscribePlayerController.BP_MindscribePlayerController_C|GetBeats_Box_Scores (Variables|Default|GetPlayer%20Controller%20Ref)) (Variables|Default|GetPlayerScore))
                (Class|LowEntryExtendedStandardLibrary|SortIntegerArrayDirectly (Variables|/Game/Blueprints/GameManagers/BP_MindscribePlayerController.BP_MindscribePlayerController_C|GetBeats_Box_Scores (Variables|Default|GetPlayer%20Controller%20Ref)) true)
                (Default|SaveBeatsBoxScore (Variables|Default|GetPlayer%20Controller%20Ref))
                (Utilities|FlowControl|Delay 3.0)
                (bind _returnvalue (UserInterface|CreateWidget "/Game/Widgets/BeatsBox/Widget_BeatsBoxScoreboard.Widget_BeatsBoxScoreboard_C"))
                (UserInterface|SetWidget (Variables|/Game/Blueprints/GameActors/BP_Screen.BP_Screen_C|GetWidget (Variables|Default|GetScreen%20Ref)) _returnvalue)))))))))

(event OnComponentEndOverlap(B_Note_Box_Collison)
  (params (OverlappedComponent :type Primitive%20Component%20Object%20Reference) (OtherActor :type Actor%20Object%20Reference) (OtherComp :type Primitive%20Component%20Object%20Reference) (OtherBodyIndex :type Integer))
  (bind _player_ref (Variables|Default|GetPlayer%20Ref))
  (if (or (== OtherComp (Variables|/Game/Blueprints/GameActors/BP_VR_Player.BP_VR_Player_C|GetMotion%20Controller%20Left%20Collision _player_ref)) (== OtherComp (Variables|/Game/Blueprints/GameActors/BP_VR_Player.BP_VR_Player_C|GetMotion%20Controller%20Right%20Collision _player_ref)))
    (if (Variables|Default|GetPlayerTurn?)
      (Utilities|FlowControl|Sequence
        (:then_0
          (Utilities|FlowControl|DoOnce false) ; enters at Reset
        )
        (:then_1
          (Rendering|Material|SetMaterial (Variables|Default|GetB_Note) 0 "/Game/Assets/Textures/M_White.M_White")
          (if (>= (Utilities|Array|Length (Variables|Default|GetPlayerAnswer)) (Utilities|Array|Length (Variables|Default|GetPianoSequence)))
            (bind _correct_ (CallFunction|CheckAnswer))
            (if _correct_
              (Variables|Default|SetPlayerTurn? false)
              (Variables|Default|SetPlayerScore (+ (Variables|Default|GetPlayerScore) 1))
              (Variables|Default|SetSequenceLength (+ (Variables|Default|GetSequenceLength) 1))
              (Utilities|Array|Clear (Variables|Default|GetPlayerAnswer))
              (Utilities|FlowControl|Delay 2.0)
              (CallFunction|PickPianoSequence)
              (else
                (Utilities|Array|Add (Variables|/Game/Blueprints/GameManagers/BP_MindscribePlayerController.BP_MindscribePlayerController_C|GetBeats_Box_Scores (Variables|Default|GetPlayer%20Controller%20Ref)) (Variables|Default|GetPlayerScore))
                (Class|LowEntryExtendedStandardLibrary|SortIntegerArrayDirectly (Variables|/Game/Blueprints/GameManagers/BP_MindscribePlayerController.BP_MindscribePlayerController_C|GetBeats_Box_Scores (Variables|Default|GetPlayer%20Controller%20Ref)) true)
                (Default|SaveBeatsBoxScore (Variables|Default|GetPlayer%20Controller%20Ref))
                (Utilities|FlowControl|Delay 3.0)
                (bind _returnvalue (UserInterface|CreateWidget "/Game/Widgets/BeatsBox/Widget_BeatsBoxScoreboard.Widget_BeatsBoxScoreboard_C"))
                (UserInterface|SetWidget (Variables|/Game/Blueprints/GameActors/BP_Screen.BP_Screen_C|GetWidget (Variables|Default|GetScreen%20Ref)) _returnvalue)))))))))

(event OnComponentEndOverlap(C_Note_Box_Collison)
  (params (OverlappedComponent :type Primitive%20Component%20Object%20Reference) (OtherActor :type Actor%20Object%20Reference) (OtherComp :type Primitive%20Component%20Object%20Reference) (OtherBodyIndex :type Integer))
  (bind _player_ref (Variables|Default|GetPlayer%20Ref))
  (if (or (== OtherComp (Variables|/Game/Blueprints/GameActors/BP_VR_Player.BP_VR_Player_C|GetMotion%20Controller%20Left%20Collision _player_ref)) (== OtherComp (Variables|/Game/Blueprints/GameActors/BP_VR_Player.BP_VR_Player_C|GetMotion%20Controller%20Right%20Collision _player_ref)))
    (if (Variables|Default|GetPlayerTurn?)
      (Utilities|FlowControl|Sequence
        (:then_0
          (Utilities|FlowControl|DoOnce false) ; enters at Reset
        )
        (:then_1
          (Rendering|Material|SetMaterial (Variables|Default|GetC_Note) 0 "/Game/Assets/Textures/M_White.M_White")
          (if (>= (Utilities|Array|Length (Variables|Default|GetPlayerAnswer)) (Utilities|Array|Length (Variables|Default|GetPianoSequence)))
            (bind _correct_ (CallFunction|CheckAnswer))
            (if _correct_
              (Variables|Default|SetPlayerTurn? false)
              (Variables|Default|SetPlayerScore (+ (Variables|Default|GetPlayerScore) 1))
              (Variables|Default|SetSequenceLength (+ (Variables|Default|GetSequenceLength) 1))
              (Utilities|Array|Clear (Variables|Default|GetPlayerAnswer))
              (Utilities|FlowControl|Delay 2.0)
              (CallFunction|PickPianoSequence)
              (else
                (Utilities|Array|Add (Variables|/Game/Blueprints/GameManagers/BP_MindscribePlayerController.BP_MindscribePlayerController_C|GetBeats_Box_Scores (Variables|Default|GetPlayer%20Controller%20Ref)) (Variables|Default|GetPlayerScore))
                (Class|LowEntryExtendedStandardLibrary|SortIntegerArrayDirectly (Variables|/Game/Blueprints/GameManagers/BP_MindscribePlayerController.BP_MindscribePlayerController_C|GetBeats_Box_Scores (Variables|Default|GetPlayer%20Controller%20Ref)) true)
                (Default|SaveBeatsBoxScore (Variables|Default|GetPlayer%20Controller%20Ref))
                (Utilities|FlowControl|Delay 3.0)
                (bind _returnvalue (UserInterface|CreateWidget "/Game/Widgets/BeatsBox/Widget_BeatsBoxScoreboard.Widget_BeatsBoxScoreboard_C"))
                (UserInterface|SetWidget (Variables|/Game/Blueprints/GameActors/BP_Screen.BP_Screen_C|GetWidget (Variables|Default|GetScreen%20Ref)) _returnvalue)))))))))

(event Custom|Pick%20Piano%20Sequence
  (Utilities|Array|Clear (Variables|Default|GetPianoSequence))
  (bind _output_get (Variables|Default|SetCurrentSequenceIndex 0))
  (if (< _output_get (Variables|Default|GetSequenceLength)) :!label _label
    (bind _returnvalue (Class|BeatsBox|PickPianoKey))
    (Utilities|Array|Add (Variables|Default|GetPianoSequence) _returnvalue)
    (switch string _returnvalue
      (:A
        (CallFunction|PlayAKey))
      (:B
        (CallFunction|PlayBKey))
      (:C
        (CallFunction|PlayCKey))
      (:D
        (CallFunction|PlayDKey)))
    (Utilities|FlowControl|Delay 3.0)
    (Variables|Default|SetCurrentSequenceIndex (+ (Variables|Default|GetCurrentSequenceIndex) 1))
    (goto _label)
    (else
      (Variables|Default|SetPlayerTurn? true))))

(event Custom|Play%20A%20Key
  (Audio|PlaySound2D "/Game/Assets/Audio/PianNotes/SoundCues/SQ_Piano_A_Note.SQ_Piano_A_Note" 1.0 1.0 0.0 0 0)
  (Rendering|Material|SetMaterial (Variables|Default|GetA_Note) 0 "/Game/Assets/Textures/M_PianoSelectedKey.M_PianoSelectedKey")
  (Utilities|FlowControl|Delay 2.0)
  (Rendering|Material|SetMaterial (Variables|Default|GetA_Note) 0 "/Game/Assets/Textures/M_White.M_White"))

(event Custom|Play%20B%20Key
  (Audio|PlaySound2D "/Game/Assets/Audio/PianNotes/SoundCues/SQ_Piano_B_Note.SQ_Piano_B_Note" 1.0 1.0 0.0 0 0)
  (Rendering|Material|SetMaterial (Variables|Default|GetB_Note) 0 "/Game/Assets/Textures/M_PianoSelectedKey.M_PianoSelectedKey")
  (Utilities|FlowControl|Delay 2.0)
  (Rendering|Material|SetMaterial (Variables|Default|GetB_Note) 0 "/Game/Assets/Textures/M_White.M_White"))

(event Custom|Play%20C%20Key
  (Audio|PlaySound2D "/Game/Assets/Audio/PianNotes/SoundCues/SQ_Piano_C_Note.SQ_Piano_C_Note" 1.0 1.0 0.0 0 0)
  (Rendering|Material|SetMaterial (Variables|Default|GetC_Note) 0 "/Game/Assets/Textures/M_PianoSelectedKey.M_PianoSelectedKey")
  (Utilities|FlowControl|Delay 2.0)
  (Rendering|Material|SetMaterial (Variables|Default|GetC_Note) 0 "/Game/Assets/Textures/M_White.M_White"))

(event Custom|Play%20D%20Key
  (Audio|PlaySound2D "/Game/Assets/Audio/PianNotes/SoundCues/SQ_Piano_D_Note.SQ_Piano_D_Note" 1.0 1.0 0.0 0 0)
  (Rendering|Material|SetMaterial (Variables|Default|GetD_Note) 0 "/Game/Assets/Textures/M_PianoSelectedKey.M_PianoSelectedKey")
  (Utilities|FlowControl|Delay 2.0)
  (Rendering|Material|SetMaterial (Variables|Default|GetD_Note) 0 "/Game/Assets/Textures/M_White.M_White"))

(event EventBeginPlay
  (bind _returnvalue (Actor|GetActorOfClass "/Game/Blueprints/GameActors/BP_Screen.BP_Screen_C"))
  (Variables|Default|SetScreen%20Ref _returnvalue)
  (bind _returnvalue_2 (Actor|GetActorOfClass "/Game/Blueprints/GameActors/BP_VR_Player.BP_VR_Player_C"))
  (Variables|Default|SetPlayer%20Ref _returnvalue_2)
  (Variables|Default|SetSequenceLength 1)
  (Variables|Default|SetPlayerScore 0)
  (bind _asbp_mindscribe_player_controller (Utilities|Casting|CastToBP_MindscribePlayerController (Game|GetPlayerController 0)))
  (Variables|Default|SetPlayer%20Controller%20Ref _asbp_mindscribe_player_controller)
  (Variables|Default|SetPlayerTurn? false)
  (Utilities|FlowControl|Delay 5.0)
  (CallFunction|PickPianoSequence))

(fn ConstructionScript)

(fn CheckAnswer
  (if (Utilities|Array|Identical (Variables|Default|GetPlayerAnswer) (Variables|Default|GetPianoSequence))
    (return true)
    (else
      (return false))))