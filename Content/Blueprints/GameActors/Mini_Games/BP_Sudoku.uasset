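; Sudoku mini-game actor that times a round and scores it for the VR player.
; Timer counts minutes and seconds through a looping one-second Delay while GameActive, then runs CalculateScore if GameWon.
; Scoring combines elapsed minutes, a lives bonus and a difficulty multiplier; as written, longer times and fewer remaining lives on Easy/Medium score higher.
; The result is shown in a Widget_Sudoku_Score placed on BP_Screen.
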(event Custom|Timer
  (Variables|Default|SetGameActive? true)
  (Variables|Default|SetMinutes 0)
  (Variables|Default|SetSeconds 0)
  (if (Variables|Default|GetGameActive?) :!label _label
    (Utilities|FlowControl|Delay 1.0)
    (bind _output_get (Variables|Default|SetSeconds (+ (Variables|Default|GetSeconds) 1)))
    (if (>= _output_get 60)
      (Variables|Default|SetMinutes (+ (Variables|Default|GetMinutes) 1))
      (Variables|Default|SetSeconds 0)
      (goto _label)
      (else
        (goto _label)))
    (elif (Variables|Default|GetGameWon?)
      (CallFunction|CalculateScore (Variables|/Game/Blueprints/GameActors/BP_VR_Player.BP_VR_Player_C|GetDifficulty (Variables|Default|GetPlayer%20Ref)) (Variables|Default|GetnumberOfLives)))))

(event Custom|Calculate%20Score
  (params (Difficulty :type String) (LivesLeft :type Integer))
  (bind _minutes (Variables|Default|GetMinutes))
  (bind _returnvalue (+ _minutes 1))
  (bind _returnvalue_2 (Math|Conversions|ToFloat(Integer) _returnvalue))
  (bind _returnvalue_3 (* 1 _returnvalue_2))
  (Variables|Default|SetLives%20Left LivesLeft)
  (Variables|Default|SetScore 1e+03)
  (switch string Difficulty
    (:Easy
      (Variables|Default|SetDifficultyBonus 0.5)
      (Variables|Default|SetLivesBonus (* (/ 5 (Variables|Default|GetLives%20Left)) 1e+02)))
    (:Medium
      (Variables|Default|SetDifficultyBonus 1.0)
      (Variables|Default|SetLivesBonus (* (/ 3 (Variables|Default|GetLives%20Left)) 1e+02)))
    (:Hard
      (Variables|Default|SetDifficultyBonus 1.0)
      (Variables|Default|SetLivesBonus (* 1 1e+02))))
  (Variables|Default|SetTimeBonus _returnvalue_3)
  (bind _output_get (Variables|Default|SetScore (* (Variables|Default|GetScore) _returnvalue_3)))
  (bind _output_get_2 (Variables|Default|SetScore (+ _output_get (Variables|Default|GetLivesBonus))))
  (Variables|Default|SetScore (* _output_get_2 (Variables|Default|GetDifficultyBonus)))
  (bind _returnvalue_4 (UserInterface|CreateWidget "/Game/Widgets/Sudoku/Widget_Sudoku_Score.Widget_Sudoku_Score_C"))
  (UserInterface|SetWidget (Variables|/Game/Blueprints/GameActors/BP_Screen.BP_Screen_C|GetWidget (Variables|Default|GetScreen%20Ref)) _returnvalue_4)
  (Default|SetScoreStats _returnvalue_4 (Variables|Default|GetTimeBonus) (Variables|/Game/Blueprints/GameActors/BP_VR_Player.BP_VR_Player_C|GetDifficulty (Variables|Default|GetPlayer%20Ref)) (Variables|Default|GetLivesBonus) (Variables|Default|GetScore)))

(event EventBeginPlay
  (bind _returnvalue (Actor|GetActorOfClass "/Game/Blueprints/GameActors/BP_VR_Player.BP_VR_Player_C"))
  (Variables|Default|SetPlayer%20Ref _returnvalue)
  (bind _returnvalue_2 (Actor|GetActorOfClass "/Game/Blueprints/GameActors/BP_Screen.BP_Screen_C"))
  (Variables|Default|SetScreen%20Ref _returnvalue_2))

(fn ConstructionScript)