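; BP_MarqueeMatchUps is a mini-game actor that holds the state of Marquee Matchups, apparently a shape-pattern matching game.
; On BeginPlay it caches references to the screen and VR player actors found by class.
; StartMarqueeMatchups resets the shape counters, the pattern, the player's answer and the score stored on BP_Screen.
; AddShapeToPattern appends a shape from PickShape to the pattern and returns it.
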(event Custom|Start%20Marquee%20Matchups
  (Variables|Default|SetCurrentShapeNumber 0)
  (Utilities|Array|Clear (Variables|Default|GetPlayerAnswer))
  (Variables|/Game/Blueprints/GameActors/BP_Screen.BP_Screen_C|SetMarqueeMatchupScore (Variables|Default|GetScreen%20Ref) 0)
  (Utilities|Array|Clear (Variables|Default|GetPattern))
  (Variables|Default|SetMaxShapes 0))

(event EventBeginPlay
  (bind _returnvalue (Actor|GetActorOfClass "/Game/Blueprints/GameActors/BP_Screen.BP_Screen_C"))
  (Variables|Default|SetScreen%20Ref _returnvalue)
  (bind _returnvalue_2 (Actor|GetActorOfClass "/Game/Blueprints/GameActors/BP_VR_Player.BP_VR_Player_C"))
  (Variables|Default|SetPlayer%20Ref _returnvalue_2))

(fn ConstructionScript)

(fn AddShapetoPattern
  (bind _returnvalue (Class|MarqueeMatchUps|PickShape))
  (Utilities|Array|Add (Variables|Default|GetPattern) _returnvalue)
  (return _returnvalue))